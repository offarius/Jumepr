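; Player pawn for an auto-running game: it moves forward constantly, steers sideways, jumps and loses below a kill height.
; The first jump press notifies BP_GameMode and plays the scale-in start timeline.
; Tick applies manual swept gravity and traces for ground; jumps use a height-lerp timeline with backpack glow.
; Leaving a BP_Floor overlap raises speed, and losing restarts through the game mode after the lose sound finishes.
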(event Custom|Jump
  (bind _mi_backpack (Variables|Default|GetMI_Backpack))
  (bind _mi_backpack_2 (Variables|Default|GetMI_Backpack))
  (bind _box (Variables|Default|GetBox))
  (bind _returnvalue (Transformation|GetWorldLocation _box))
  (if (Variables|Default|GetOnGround)
    (Audio|SpawnSoundAttached "/Game/SFX/MS_Jump.MS_Jump" (Variables|Default|GetBox) "None" "0, 0, 0" "0, 0, 0" "KeepRelativeOffset" false 1.0 1.0 0.0 0 0)
    (Variables|Default|SetGroundLevel (.z (Transformation|GetActorLocation)))
    (bind _heightalpha (Timeline|JumpAlpha PlayFromStart)
      (:Update
        (Transformation|SetWorldLocation _box (Math|Vector|MakeVector (.x _returnvalue) (.y _returnvalue) (Math|Float|Lerp (Variables|Default|GetGroundLevel) (+ (Variables|Default|GetGroundLevel) (Variables|Default|GetJumpHeight)) _heightalpha)) true false)
        (Rendering|Material|SetScalarParameterValue _mi_backpack_2 "HeatColorAlpha" 1.0 :!class /Script/Engine.MaterialInstanceDynamic)
        (Rendering|Material|SetScalarParameterValue _mi_backpack_2 "Glow" 5e+01 :!class /Script/Engine.MaterialInstanceDynamic))
      (:Finished
        (Rendering|Material|SetScalarParameterValue _mi_backpack "HeatColorAlpha" 0.0 :!class /Script/Engine.MaterialInstanceDynamic)
        (Rendering|Material|SetScalarParameterValue _mi_backpack "Glow" 1.0 :!class /Script/Engine.MaterialInstanceDynamic)))))

(event Custom|Loose
  ;[0.15 0.15 0.15 0.5] Restart
  (Utilities|FlowControl|DoOnce false
    (:Completed
      (bind _returnvalue (Audio|SpawnSoundAttached "/Game/SFX/MS_Lose.MS_Lose" (Variables|Default|GetBox) "None" "0, 0, 0" "0, 0, 0" "KeepRelativeOffset" false 1.0 1.0 0.0 0 0))
      (EventDispatchers|AssignOnAudioFinished _returnvalue (delegate Custom|OnAudioFinished_Event)))))

(event Custom|IncreasePlayerSpeed
  (bind _floatingpawnmovement (Variables|Default|GetFloatingPawnMovement))
  ;[0.15 0.15 0.15 0.5] Увеличение скорости
  (Variables|/Script/Engine.FloatingPawnMovement|SetMaxSpeed _floatingpawnmovement (+ (Class|MovementComponent|GetMaxSpeed _floatingpawnmovement) (Variables|Default|GetSpeedUp))))

(event Custom|PlayStartAnim
  (Audio|SpawnSoundAttached "/Game/SFX/MS_Start.MS_Start" (Variables|Default|GetBox) "None" "0, 0, 0" "0, 0, 0" "KeepRelativeOffset" false 1.0 1.0 0.0 0 0)
  (bind (_direction _xyscale _zscale _fallalpha) (Timeline|StartTimeline PlayFromStart)
    (:Update
      (Transformation|SetActorScale3D (Math|Vector|MakeVector _xyscale _xyscale _zscale))
      (Variables|Default|SetFallSpeed (Math|Float|Lerp 0.0 1e+02 _fallalpha))
      (Transformation|AddLocalRotation (Variables|Default|GetStaticMesh) "0.000000,90.000000,0.000000" false false))
    (:Finished
      (Variables|Default|SetFallSpeed 1.5e+03)
      (Transformation|SetWorldRotation (Variables|Default|GetStaticMesh) "0.000000,90.000000,0.000000" false false)
      (Variables|Default|SetBReady true))))

(event Custom|OnAudioFinished_Event
  (Actor|DestroyActor)
  (bind _asbp_game_mode (Utilities|Casting|CastToBP_GameMode (Game|GetGameMode)))
  (Default|CallRestart _asbp_game_mode))

(event Input|EnhancedActionEvents|EnhancedInputActionIA_MoveRight
  (params (ActionValue :type Float%20%28double-precision%29) (ElapsedSeconds :type Float%20%28double-precision%29) (TriggeredSeconds :type Float%20%28double-precision%29) (InputAction :type Input%20Action%20Object%20Reference :default "/Game/Input/Actions/IA_MoveRight.IA_MoveRight"))
  ;[0.15 0.15 0.15 0.5] Движение в стороны
  (if (Variables|Default|GetBReady)
    (Pawn|Input|AddMovementInput (Math|Vector|GetRightVector (Variables|Default|GetBox)) ActionValue false)))

(event Input|EnhancedActionEvents|EnhancedInputActionIA_Jump
  (params (ActionValue :type Boolean) (ElapsedSeconds :type Float%20%28double-precision%29) (TriggeredSeconds :type Float%20%28double-precision%29) (InputAction :type Input%20Action%20Object%20Reference :default "/Game/Input/Actions/IA_Jump.IA_Jump"))
  (:Started
    (if (Variables|Default|GetBReady)
      (CallFunction|Jump)
      (else
        (Default|CallPlayerReady (.AsBP%20Game%20Mode (Utilities|Casting|CastToBP_GameMode (Game|GetGameMode))))
        (CallFunction|PlayStartAnim)))))

(event EventTick
  (params (DeltaSeconds :type Float%20%28single-precision%29))
  (bind _box (Variables|Default|GetBox))
  (bind _returnvalue (Transformation|GetWorldLocation _box))
  (Transformation|AddActorWorldOffset (* (Math|Vector|NegateVector (Math|Vector|GetUpVector (Variables|Default|GetBox))) (* (Variables|Default|GetFallSpeed) (Utilities|Time|GetWorldDeltaSeconds))) true)
  (if (Variables|Default|GetBReady)
    ;[0.15 0.15 0.15 0.5] Restart
    (if (> (.z (Transformation|GetActorLocation)) (Variables|Default|GetKillVoidZ))
      (Utilities|FlowControl|Sequence
        (:then_0
          (Pawn|Input|AddMovementInput (Math|Vector|GetForwardVector (Variables|Default|GetBox)) 1.0 false))
        (:then_1
          (bind _returnvalue_2 (Collision|LineTraceByChannel _returnvalue (+ _returnvalue (* (Math|Vector|NegateVector (Math|Vector|GetUpVector _box)) 5e+01)) "TraceTypeQuery1" false 0 "None"))
          (Variables|Default|SetOnGround _returnvalue_2)))
      (else
        (CallFunction|Loose)))))

(event Collision|EventActorEndOverlap
  (params (OtherActor :type Actor%20Object%20Reference))
  ;[0.15 0.15 0.15 0.5] Увеличение скорости
  (Utilities|Casting|CastToBP_Floor OtherActor)
  (CallFunction|IncreasePlayerSpeed)
  (Default|CallSpeedIncrease (.AsBP%20Game%20Mode (Utilities|Casting|CastToBP_GameMode (Game|GetGameMode)))))

(event EventBeginPlay
  (Utilities|FlowControl|Sequence
    (:then_0
      (Transformation|SetActorScale3D "0.000100,0.000100,0.000100"))
    (:then_1
      (bind _returnvalue (Rendering|Material|CreateDynamicMaterialInstance (Variables|Default|GetStaticMesh) 1 "/Game/Assests/Character/Materials/MI_OrangeBackpack.MI_OrangeBackpack" "None" :!class /Script/Engine.PrimitiveComponent))
      (Variables|Default|SetMI_Backpack _returnvalue))))

(fn ConstructionScript)