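; Environment manager that builds a looping track from pooled floor platforms and decorative rocks.
; On BeginPlay it spawns the floors and both rock pools, and binds a floor-move event.
; That event shifts the ready floor ahead by the track length, respawns its cubes and repositions rocks beside it.
; Big rocks cycle through their pool, while the small-rock counter's inverted wrap check keeps reusing the first two.
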(event Custom|SpawnFloor
  (for _index (range 0 (- (Variables|Default|GetPlatformNum) 1))
    (bind _returnvalue (Game|SpawnActorfromClass "/Game/Blueprints/BP_Floor.BP_Floor_C" (Math|Transform|MakeTransform (Math|Vector|MakeVector (* (CallFunction|GetPlatformOffset) _index) 0.0 0.0) "0, 0, 0" "1.000000,1.000000,1.000000") "Undefined" "MultiplyWithRoot" 0 (Variables|Default|GetNum%20X) (Variables|Default|GetNum%20Y) (Variables|Default|GetOffset) 0))
    (Utilities|Array|Add (Variables|Default|GetFloorArray) _returnvalue)
    (Default|SpawnCubes _returnvalue)))

(event Custom|BPMoveFloor
  (params (ReadyFloor :type BP%20Floor%20Object%20Reference))
  (bind _returnvalue (Transformation|GetActorLocation ReadyFloor))
  (bind _platformoffset (CallFunction|GetPlatformOffset))
  (bind _platformnum (Variables|Default|GetPlatformNum))
  (bind _returnvalue_2 (* _platformoffset _platformnum))
  (bind _returnvalue_3 (+ _returnvalue_2 (.x _returnvalue)))
  (Utilities|IsValid ReadyFloor
    (:Is%20Valid
      (Transformation|SetActorLocation ReadyFloor (Math|Vector|MakeVector _returnvalue_3 (.y _returnvalue) (.z _returnvalue)) false false)
      (Default|SpawnCubes ReadyFloor)
      (CallFunction|MoveBigRock _returnvalue_3)
      (CallFunction|MoveSmallRocks _returnvalue_3))))

(event Custom|SpawnBigRocks
  (for _index (range 0 (Variables|Default|GetObjectCount))
    (bind _returnvalue (Game|SpawnActorfromClass "/Game/Blueprints/BP_BigRock.BP_BigRock_C" (Math|Transform|MakeTransform "-8000.000000,0.000000,0.000000" "0, 0, 0" "16.000000,16.000000,16.000000") "Undefined" "MultiplyWithRoot" 0 0))
    (Utilities|Array|Add (Variables|Default|GetBigRockArray) _returnvalue)))

(event Custom|SpawnSmallRock
  (for _index (range 0 (Variables|Default|GetObjectCount))
    (bind _returnvalue (Game|SpawnActorfromClass "/Game/Blueprints/BP_SmallRock.BP_SmallRock_C" (Math|Transform|MakeTransform "-8000.000000,0.000000,0.000000" "0, 0, 0" "3.000000,3.000000,3.000000") "Undefined" "MultiplyWithRoot" 0 0))
    (Utilities|Array|Add (Variables|Default|GetSmallRocksArray) _returnvalue)))

(event Custom|MoveBigRock
  (params (PlatformX :type Float%20%28double-precision%29))
  (if (>= (Variables|Default|GetBigRocksCounter) (Utilities|Array|LastIndex (Variables|Default|GetBigRockArray)))
    (Variables|Default|SetBigRocksCounter 0))
  (Utilities|FlowControl|Sequence
    (:then_0
      (Default|MoveRock (Utilities|Array|Get(acopy) (Variables|Default|GetBigRockArray) (Variables|Default|GetBigRocksCounter)) (Math|Vector|MakeVector (+ PlatformX 1e+03) -3.2e+03 -4e+03))
      (Math|Integer|IncrementInt (Variables|Default|GetBigRocksCounter)))
    (:then_1
      (Default|MoveRock (Utilities|Array|Get(acopy) (Variables|Default|GetBigRockArray) (Variables|Default|GetBigRocksCounter)) (Math|Vector|MakeVector (- PlatformX 1e+03) 1.5e+03 -1e+03))
      (Math|Integer|IncrementInt (Variables|Default|GetBigRocksCounter)))))

(event Custom|MoveSmallRocks
  (params (PlatformX :type Float%20%28double-precision%29))
  (if (>= (Utilities|Array|LastIndex (Variables|Default|GetSmallRocksArray)) (Variables|Default|GetSmallRocksCounter))
    (Variables|Default|SetSmallRocksCounter 0))
  (Utilities|FlowControl|Sequence
    (:then_0
      (Default|MoveStone (Utilities|Array|Get(acopy) (Variables|Default|GetSmallRocksArray) (Variables|Default|GetSmallRocksCounter)) (Math|Vector|MakeVector (+ PlatformX (Math|Random|RandomFloatinRange 1e+02 5e+02)) (Math|Random|RandomFloatinRange -1.5e+02 -2e+02) -5e+01))
      (Math|Integer|IncrementInt (Variables|Default|GetSmallRocksCounter)))
    (:then_1
      (Default|MoveStone (Utilities|Array|Get(acopy) (Variables|Default|GetSmallRocksArray) (Variables|Default|GetSmallRocksCounter)) (Math|Vector|MakeVector (+ PlatformX (Math|Random|RandomFloatinRange 1e+02 5e+02)) (Math|Random|RandomFloatinRange 3.3e+02 3.5e+02) 5e+01))
      (Math|Integer|IncrementInt (Variables|Default|GetSmallRocksCounter)))))

(event EventBeginPlay
  (Utilities|FlowControl|Sequence
    (:then_0
      (CallFunction|SpawnFloor))
    (:then_1
      (EventDispatchers|BindEventtoMoveFloor (EventDispatchers|CreateEvent :!event Custom|BPMoveFloor)))
    (:then_2
      (CallFunction|SpawnBigRocks))
    (:then_3
      (CallFunction|SpawnSmallRock))))

(fn ConstructionScript)

(fn GetPlatformOffset
  (return (* (Variables|Default|GetOffset) (+ (Variables|Default|GetNum%20X) 1))))