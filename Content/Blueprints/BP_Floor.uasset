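; BP_Floor is a floor segment that spawns a grid of BP_Cube actors, tagging edge cubes by position, under a trigger fitted to the grid at construction.
; When BP_Pawn enters, it randomly calls obstacle generation on cubes in the last rows, then drops all cubes with row-staggered random ranges and clears the array.
; When the pawn leaves, it asks BP_EnvManager to move the floor.
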(event Custom|SpawnCubes
  (bind _defaultsceneroot (Variables|Default|GetDefaultSceneRoot))
  (bind _returnvalue (Transformation|GetWorldLocation _defaultsceneroot))
  (for _index (range 0 (Variables|Default|GetNumX))
    (bind _returnvalue_2 (Utilities|Array|Add :TargetArray (Variables|Default|GetBlockArray)))
    (for _index_2 (range 0 (Variables|Default|GetNumY))
      (bind _returnvalue_3 (Game|SpawnActorfromClass "/Game/Blueprints/BP_Cube.BP_Cube_C" (Math|Transform|MakeTransform (Math|Vector|MakeVector (+ (* (Variables|Default|GetOffset) _index) (.x _returnvalue)) (+ (* (Variables|Default|GetOffset) _index_2) (.y _returnvalue)) (.z _returnvalue)) "0, 0, 0" "1.000000,1.000000,1.000000") "Undefined" "MultiplyWithRoot" 0 (CallFunction|CheckCubePos _index_2) 0))
      (Utilities|Array|Add (Utilities|Struct|BreakBlocksRow (Utilities|Array|Get(acopy) (Variables|Default|GetBlockArray) _returnvalue_2)) _returnvalue_3))))

(event Custom|DropCubes
  (for (_array_element _array_index) (Variables|Default|GetBlockArray)
    (for _array_element_2 (Utilities|Struct|BreakBlocksRow _array_element)
      (Utilities|IsValid _array_element_2
        (:Is%20Valid
          (Default|Fall _array_element_2 (+ (* _array_index 0.2) 0.1) (+ (* _array_index 0.2) 0.5))))))
  (Utilities|Array|Clear (Variables|Default|GetBlockArray)))

(event Custom|SpawnObst
  (bind _blockarray (Variables|Default|GetBlockArray))
  (for _index (range 0 (Math|Random|RandomIntegerinRange 0 (Variables|Default|GetRowsObst)))
    (for _array_element (Utilities|Struct|BreakBlocksRow (Utilities|Array|Get(acopy) _blockarray (- (Utilities|Array|LastIndex _blockarray) _index)))
      (Utilities|IsValid _array_element
        (:Is%20Valid
          (if (Math|Random|RandomBoolwithWeight 0.7)
            (Default|RandomObst _array_element)))))))

(event EventBeginPlay
  (bind _returnvalue (Actor|GetActorOfClass "/Game/Blueprints/BP_EnvManager.BP_EnvManager_C"))
  (Utilities|IsValid _returnvalue
    (:Is%20Valid
      (Variables|Default|SetEnv%20Manager _returnvalue))))

(event Collision|EventActorBeginOverlap
  (params (OtherActor :type Actor%20Object%20Reference))
  (Utilities|Casting|CastToBP_Pawn OtherActor)
  (Utilities|FlowControl|Sequence
    (:then_0
      (CallFunction|SpawnObst))
    (:then_1
      (CallFunction|DropCubes))))

(event Collision|EventActorEndOverlap
  (params (OtherActor :type Actor%20Object%20Reference))
  (Utilities|Casting|CastToBP_Pawn OtherActor)
  (Default|CallMoveFloor (Variables|Default|GetEnv%20Manager) self))

(fn ConstructionScript
  (bind _trigger (Variables|Default|GetTrigger))
  (bind _defaultsceneroot (Variables|Default|GetDefaultSceneRoot))
  (bind _returnvalue (Transformation|GetWorldLocation _defaultsceneroot))
  (Transformation|SetWorldLocation _trigger (Math|Vector|MakeVector (+ (.x _returnvalue) (Math|Float|SafeDivide (* (Variables|Default|GetOffset) (Variables|Default|GetNumX)) 2.0)) (+ (.y _returnvalue) (Math|Float|SafeDivide (* (Variables|Default|GetOffset) (Variables|Default|GetNumY)) 2.0)) (+ (Math|Float|SafeDivide (Variables|Default|GetOffset) 2.0) (.z _returnvalue))) false false)
  (Transformation|SetWorldScale3D _trigger (Math|Vector|MakeVector (Math|Conversions|ToFloat(Integer) (+ (Variables|Default|GetNumX) 1)) (Math|Conversions|ToFloat(Integer) (+ (Variables|Default|GetNumY) 2)) 1.0)))

(fn CheckCubePos
  (params (Index :type Integer))
  (if (== Index 0)
    (return "NewEnumerator0")
    (elif (== Index (Variables|Default|GetNumY))
      (return "NewEnumerator2")
      (else
        (return "NewEnumerator1")))))