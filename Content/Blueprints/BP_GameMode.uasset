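; Game mode that handles level restart, background music and fog color feedback for player speed increases.
; On BeginPlay it binds restart, speed increase and player ready events, caches the level's ExponentialHeightFog and starts the music.
; Each speed-up shifts the fog inscattering color toward red within clamped limits, while restart reopens the Test level.
; The start-game handler is empty.
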(event Custom|RestartGame
  (Game|OpenLevel(byObjectReference) "/Game/Maps/Test.Test"))

(event Custom|PlayerSpeedUp
  (bind _fogcolorchangeeffect (Variables|Default|GetFogColorChangeEffect))
  (bind _output_get (Variables|Default|SetCurrentColor (Utilities|Struct|MakeLinearColor (Math|Float|Min(Float) (+ (.r (Variables|Default|GetCurrentColor)) _fogcolorchangeeffect) 0.5) (Math|Float|Max(Float) (- (.g (Variables|Default|GetCurrentColor)) _fogcolorchangeeffect) 0.02) (Math|Float|Max(Float) (- (.b (Variables|Default|GetCurrentColor)) _fogcolorchangeeffect) 0.04) (.a (Variables|Default|GetCurrentColor)))))
  (Class|ExponentialHeightFogComponent|SetFogInscatteringColor (Variables|/Script/Engine.ExponentialHeightFog|GetComponent (Variables|Default|GetLevelFog)) _output_get))

(event Custom|StaartGame)

(event EventBeginPlay
  (Utilities|FlowControl|Sequence
    (:then_0
      (EventDispatchers|BindEventtoRestart (EventDispatchers|CreateEvent :!event Custom|RestartGame)))
    (:then_1
      (EventDispatchers|BindEventtoSpeedIncrease (EventDispatchers|CreateEvent :!event Custom|PlayerSpeedUp)))
    (:then_2
      (EventDispatchers|BindEventtoPlayerReady (EventDispatchers|CreateEvent :!event Custom|StaartGame)))
    (:then_3
      (bind _returnvalue (Actor|GetActorOfClass "/Script/Engine.ExponentialHeightFog"))
      (Utilities|IsValid _returnvalue
        (:Is%20Valid
          (Variables|Default|SetLevelFog _returnvalue)
          (Variables|Default|SetCurrentColor (Variables|Default|GetBaseFogColor)))))
    (:then_4
      (Audio|Components|Audio|Play (Variables|Default|GetMusic) 0.0))))

(fn ConstructionScript)